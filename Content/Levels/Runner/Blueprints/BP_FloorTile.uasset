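; Floor tile for an endless runner level that builds its own contents and keeps the track extending.
; The construction script adds child actors: alternating left and right footsteps, random obstacles at preset spawn points, and coins scattered within CoinArea.
; When RehabCharacter overlaps the Box trigger, the tile asks RunnerGameMode to add another tile, then destroys itself after a short delay.
; GetAttachTransform exposes the AttachPoint world transform.
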(event `self.Box.OnComponentBeginOverlap`
  (params (OverlappedComponent :type "PrimitiveComponent Object Reference") (OtherActor :type "Actor Object Reference") (OtherComp :type "PrimitiveComponent Object Reference") (OtherBodyIndex :type Integer) (bFromSweep :type Boolean) (SweepResult :type "HitResult Structure (by ref)"))
  (cast `/Game/ROSIntegrationContent/RehabCharacter` OtherActor)
  (bind _asrunner_game_mode (cast `/Game/Levels/Runner/Blueprints/RunnerGameMode` (`GameplayStatics.GetGameMode`)))
  (`/Game/Levels/Runner/Blueprints/RunnerGameMode.AddFloorTile` _asrunner_game_mode)
  (`KismetSystemLibrary.Delay` 2.0)
  (`self.K2_DestroyActor`))

(fn `GetAttachTransform`
  (returns (AttachTransform :type "Transform Structure"))
  (return (`SceneComponent.K2_GetComponentToWorld` (`self.AttachPoint`))))

(fn `SetFootstepPoints`
  (bind _footsteppoints (`self.FootstepPoints`))
  (bind (_returnvalue_location _returnvalue_rotation) (`KismetMathLibrary.BreakTransform` (`SceneComponent.GetRelativeTransform` (`self.DefaultSceneRoot`))))
  (bind _y (.y _returnvalue_location))
  (bind _returnvalue (+ (.z _returnvalue_location) 15.0))
  (for _index (range 5)
    (bind _returnvalue_2 (* _index 200.0))
    (`KismetArrayLibrary.Array_Add` _footsteppoints (`KismetMathLibrary.MakeTransform` (`KismetMathLibrary.MakeVector` (+ _returnvalue_2 50.0) (+ _y 75.0) _returnvalue) _returnvalue_rotation))
    (`KismetArrayLibrary.Array_Add` _footsteppoints (`KismetMathLibrary.MakeTransform` (`KismetMathLibrary.MakeVector` (+ _returnvalue_2 150.0) (+ _y -75.0) _returnvalue) _returnvalue_rotation)))
  (return))

(fn `SetSpawnPoints`
  (set `self.SpawnPoints` (`|MakeArray` (`SceneComponent.GetRelativeTransform` (`self.SpawnPointM`)) (`SceneComponent.GetRelativeTransform` (`self.SpawnPointR0`)) (`SceneComponent.GetRelativeTransform` (`self.SpawnPointR1`)) (`SceneComponent.GetRelativeTransform` (`self.SpawnPointL0`)) (`SceneComponent.GetRelativeTransform` (`self.SpawnPointL1`)))))

(fn `SpawnCoins`
  (bind _coinarea (`self.CoinArea`))
  (bind (_returnvalue_x _returnvalue_y) (`KismetMathLibrary.BreakVector` (`KismetMathLibrary.RandomPointInBoundingBox` (`SceneComponent.RelativeLocation` _coinarea) (`BoxComponent.BoxExtent` _coinarea))))
  (for _ (range 4)
    (`AddComponent|NODE_AddChildActorComponent-1` :`RelativeTransform` (`KismetMathLibrary.Conv_VectorToTransform` (`KismetMathLibrary.MakeVector` _returnvalue_x _returnvalue_y 60.0)))))

(fn `SpawnFootsteps`
  (for (_array_element _array_index) (`self.FootstepPoints`)
    (`AddComponent|NODE_AddChildActorComponent-4` :`RelativeTransform` _array_element)
    (if (`KismetMathLibrary.Conv_IntToBool` (mod _array_index 2))
      _)))

(fn `SpawnObstacle`
  (bind _spawnpoints (`self.SpawnPoints`))
  (`AddComponent|NODE_AddChildActorComponent-0` :`RelativeTransform` (`|GetArrayItem` _spawnpoints (`KismetMathLibrary.RandomIntegerInRange` 0 (`KismetArrayLibrary.Array_LastIndex` _spawnpoints)))))

(fn `UserConstructionScript`
  (`self.SetFootstepPoints`)
  (`self.SpawnFootsteps`)
  (`self.SetSpawnPoints`)
  (for _ (range (+ (`KismetMathLibrary.RandomIntegerInRange` -1 2) 1))
    (`self.SpawnObstacle`))
  (`self.SpawnCoins`))