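; Game mode for a runner level that builds the floor from chained tiles and keeps the coin count.
; On BeginPlay it shows the run HUD and spawns an initial stretch of floor tiles.
; AddFloorTile spawns each tile at the stored next spawn point, then takes that tile's attach transform as the following one.
; AddCoin increments the counter and only prints the total as debug text.
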(event `self.ReceiveBeginPlay`
  (bind _returnvalue (`|CreateWidget` "/Game/Levels/Runner/HUD/RunHUD.RunHUD_C"))
  (`UserWidget.AddToViewport` _returnvalue 0)
  (for _ (range 10)
    (`self.AddFloorTile`)))

(fn `AddCoin`
  (bind _output_get (set `self.CoinCounter` (+ (`self.CoinCounter`) 1)))
  (`KismetSystemLibrary.PrintString` (`KismetStringLibrary.Concat_StrStr` "Current coins: " (`KismetStringLibrary.Conv_IntToString` _output_get))))

(fn `AddFloorTile`
  (bind _returnvalue (`|SpawnActorFromClass` "/Game/Levels/Runner/Blueprints/BP_FloorTile.BP_FloorTile_C" (`self.NextSpawnPoint`) "Undefined" "OverrideRootScale" null null))
  (bind _asbp_floor_tile (cast `/Game/Levels/Runner/Blueprints/BP_FloorTile` _returnvalue))
  (bind _attachtransform (`/Game/Levels/Runner/Blueprints/BP_FloorTile.GetAttachTransform` _asbp_floor_tile))
  (set `self.NextSpawnPoint` _attachtransform))

(fn `UserConstructionScript`)