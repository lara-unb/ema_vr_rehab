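; Blueprint actor that mirrors the orientation of a lower-right-leg IMU in the scene.
; On BeginPlay it caches the first TCPSocketerActor found.
; Each Tick it looks up the "lowerRightLeg" quaternion in that actor's orientation map, converts it to Euler angles and sets its own rotation with a fixed yaw offset.
; ROS topic subscription and a rotation relative to the upper leg remain as unconnected nodes.
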(event `self.ReceiveBeginPlay`
  (bind _outactors (`GameplayStatics.GetAllActorsOfClass` "/Game/Network/SocketActors/TCPSocketerActor.TCPSocketerActor_C"))
  (set `self.TCPReference` (`|GetArrayItem` _outactors)))

(event `self.ReceiveTick`
  (params (DeltaSeconds :type "Float (single-precision)"))
  (bind _astcpsocketer_actor (cast `/Game/Network/SocketActors/TCPSocketerActor` (`self.TCPReference`)))
  (`/Engine/EditorBlueprintResources/StandardMacros.IsValid` _astcpsocketer_actor
    (:`Is Valid`
      (if true
        (bind _returnvalue (`BlueprintQuaternionLibrary.Euler` (`BlueprintMapLibrary.Map_Find` (`/Game/Network/SocketActors/TCPSocketerActor.OrientationQuatMap` _astcpsocketer_actor) "lowerRightLeg")))
        (bind _output_get (set `self.OrientationMap` _returnvalue))
        (`self.K2_SetActorRotation` (`KismetMathLibrary.MakeRotator` (- (.x _output_get) 0.0) (- (.y _output_get) 0.0) (- (.z _output_get) 180.0)))))))

(fn `UserConstructionScript`)